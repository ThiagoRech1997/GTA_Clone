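; Health component that manages the player character's health and damage feedback, operating on player 0's character cached at BeginPlay.
; SetDamage plays a camera shake and explosion emitter at the mesh, then subtracts health clamped at zero through SetHealth, only when OnlyHealth is set.
; SetHealth adds up to MaxHealth or overwrites, messages the AnimInstance whether health is at or below MinHealth, and slows walk speed when it is, without restoring it.
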(event `self.ReceiveBeginPlay`
  ;[1 1 1] Event Begin Play
  (set `self.Character` (`GameplayStatics.GetPlayerCharacter` 0)))

(event `self.setHealth`
  (params (AddHealth :type Boolean) (NewHealth :type "Float (double-precision)"))
  (bind _character (`self.Character`))
  (bind _returnvalue (<= (`self.Health`) (`self.MinHealth`)))
  (bind _charactermovement (`Character.CharacterMovement` _character))
  ;[1 1 1] Life System
  (if AddHealth
    (set `self.Health` (`KismetMathLibrary.FMin` (+ (`self.Health`) NewHealth) (`self.MaxHealth`)))
    (else
      (set `self.Health` NewHealth)))
  (message `/Game/Blueprints/BP_CharacterInterface.DamageAnimation` (`SkeletalMeshComponent.GetAnimInstance` (`Character.Mesh` _character)) _returnvalue)
  (set `CharacterMovementComponent.MaxWalkSpeed` (select `bool` _returnvalue :`false` (`CharacterMovementComponent.MaxWalkSpeed` _charactermovement) :`true` 150.0) _charactermovement))

(event `self.SetDamage`
  (params (Damage :type "Float (double-precision)") (OnlyHealth :type Boolean))
  (bind _returnvalue (- (`self.Health`) (`self.Damage`)))
  ;[1 1 1] Damage System / Damage Effect
  (set `self.Damage` Damage)
  (`PlayerCameraManager.StartCameraShake` :`self` (`GameplayStatics.GetPlayerCameraManager` 0) :`ShakeClass` "/Game/Blueprints/CameraEffects/Damage_CS.Damage_CS_C" :`Scale` 0.1)
  (`GameplayStatics.SpawnEmitterAtLocation` "/Game/StarterContent/Particles/P_Explosion.P_Explosion" (`SceneComponent.GetSocketLocation` (`Character.Mesh` (`self.Character`)) "None"))
  (if OnlyHealth
    (if (<= _returnvalue 0.0)
      (`self.setHealth` false)
      (else
        (`self.setHealth` false _returnvalue)))))